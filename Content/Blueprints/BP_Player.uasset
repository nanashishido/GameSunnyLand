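; BP_Player is the playable 2D flipbook character, driven by Enhanced Input for running and jumping.
; BeginPlay adds the default mapping context, and movement input moves along the actor's forward vector, swaps run/idle flipbooks and rotates the sprite by direction.
; Jumping sets a flag that blocks movement and repeat jumps, plays the jump flipbook, then polls vertical velocity through a delay loop until zero restores idle.
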(event `self.ReceiveBeginPlay`
  (bind _asbp_player_controler (cast `/Game/Blueprints/BP_PlayerControler` (`self.GetController`)))
  (`EnhancedInputSubsystemInterface.AddMappingContext` (pcsubsystem `EnhancedInputLocalPlayerSubsystem` _asbp_player_controler) "/Game/Blueprints/IMC_default.IMC_default" 0 (struct)))

(event `EnhancedInput|/Game/Blueprints/IA_Movement`
  (params (ActionValue :type "Float (double-precision)") (ElapsedSeconds :type "Float (double-precision)") (TriggeredSeconds :type "Float (double-precision)") (InputAction :type "InputAction Object Reference" :default "/Game/Blueprints/IA_Movement.IA_Movement"))
  (:`Triggered`
    (if (not (`self.BlsJumping`))
      (`self.AddMovementInput` (`self.GetActorForwardVector`) ActionValue)
      (`PaperFlipbookComponent.SetFlipbook` (`self.Sprite`) "/Game/Assets/FB_run.FB_run")
      (if (> ActionValue 0.0)
        (`SceneComponent.K2_SetWorldRotation` :`self` (`self.Sprite`))
        (else
          (`SceneComponent.K2_SetWorldRotation` (`self.Sprite`) (struct :`Yaw` -180.0) false false)))))
  (:`Completed`
    (if (not (`self.BlsJumping`))
      (`PaperFlipbookComponent.SetFlipbook` (`self.Sprite`) "/Game/Assets/FB_idel.FB_idel"))))

(event `EnhancedInput|/Game/Blueprints/IA_Jump`
  (params (ActionValue :type Boolean) (ElapsedSeconds :type "Float (double-precision)") (TriggeredSeconds :type "Float (double-precision)") (InputAction :type "InputAction Object Reference" :default "/Game/Blueprints/IA_Jump.IA_Jump"))
  (bind _sprite (`self.Sprite`))
  (:`Triggered`
    (if (not (`self.BlsJumping`))
      (set `self.BlsJumping` true)
      (`self.Jump`)
      (`PaperFlipbookComponent.SetLooping` _sprite false)
      (`PaperFlipbookComponent.SetFlipbook` _sprite "/Game/Assets/FB_jump.FB_jump")
      (`KismetSystemLibrary.Delay` 0.2)
      (if (== (.z (`self.GetVelocity`)) 0.0) :!label _label
        (`PaperFlipbookComponent.SetLooping` _sprite false)
        (`PaperFlipbookComponent.Play` _sprite)
        (`PaperFlipbookComponent.SetFlipbook` _sprite "/Game/Assets/FB_idel.FB_idel")
        (set `self.BlsJumping` false)
        (else
          (`KismetSystemLibrary.Delay` 0.1)
          (goto _label))))))

(fn `UserConstructionScript`)